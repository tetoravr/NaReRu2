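; Subway platform screen door (home door) with two sliding panels that open and close through custom events.
; HomeDoorOpen plays a timeline that drives the right panel's relative Y position and applies the negated value to the left panel.
; HomeDoorClose reverses that timeline, while already_Open snaps both panels to fixed open offsets without touching the timeline.
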(event Custom|HomeDoorOpen
  (bind _新規track_1 (Timeline|タイムライン_0 Play)
    (:Update
      (Transformation|SetRelativeLocation (Variables|Default|Gethome_door_homedoor_Door_R) (Math|Vector|MakeVector 0.0 _新規track_1 0.0) false false)
      (Transformation|SetRelativeLocation (Variables|Default|Gethome_door_homedoor_Door_L) (Math|Vector|MakeVector 0.0 (* _新規track_1 -1.0) 0.0) false false))))

(event Custom|HomeDoorClose
  (bind _新規track_1 (Timeline|タイムライン_0 Reverse)
    (:Update
      (Transformation|SetRelativeLocation (Variables|Default|Gethome_door_homedoor_Door_R) (Math|Vector|MakeVector 0.0 _新規track_1 0.0) false false)
      (Transformation|SetRelativeLocation (Variables|Default|Gethome_door_homedoor_Door_L) (Math|Vector|MakeVector 0.0 (* _新規track_1 -1.0) 0.0) false false))))

(event Custom|already_Open
  (Transformation|SetRelativeLocation (Variables|Default|Gethome_door_homedoor_Door_R) (Math|Vector|MakeVector 0.0 -1e+02 0.0) false false)
  (Transformation|SetRelativeLocation (Variables|Default|Gethome_door_homedoor_Door_L) (Math|Vector|MakeVector 0.0 (* -1e+02 -1.0) 0.0) false false))

(fn ConstructionScript)