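; Subway train Blueprint that opens and closes sliding doors on its left and right sides.
; Separate open and close events for each side drive that side's own Timeline, playing from the start to open and reversing from the end to close.
; Each Timeline's track value sets the relative X of two door components, negated for one so the pair slides in opposite directions.
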(event Custom|Open_Door_Train_R
  ;[1 1 1] 電車右
  (bind _新規track_0 (Timeline|タイムライン_0 PlayFromStart)
    (:Update
      (Transformation|SetRelativeLocation (Variables|Default|Gettrain_0309_doorRR) (Math|Vector|MakeVector _新規track_0 0.0 0.0) false false)
      (Transformation|SetRelativeLocation (Variables|Default|Gettrain_0309_doorRL) (Math|Vector|MakeVector (* _新規track_0 -1.0) 0.0 0.0) false false))))

(event Custom|Close_Door_Train_R
  ;[1 1 1] 電車右
  (bind _新規track_0 (Timeline|タイムライン_0 ReverseFromEnd)
    (:Update
      (Transformation|SetRelativeLocation (Variables|Default|Gettrain_0309_doorRR) (Math|Vector|MakeVector _新規track_0 0.0 0.0) false false)
      (Transformation|SetRelativeLocation (Variables|Default|Gettrain_0309_doorRL) (Math|Vector|MakeVector (* _新規track_0 -1.0) 0.0 0.0) false false))))

(event Custom|Open_Door_L
  ;[1 1 1] 電車左
  (bind _新規track_0 (Timeline|タイムライン_2 PlayFromStart)
    (:Update
      (Transformation|SetRelativeLocation (Variables|Default|Gettrain_0309_doorLL) (Math|Vector|MakeVector _新規track_0 0.0 0.0) false false)
      (Transformation|SetRelativeLocation (Variables|Default|Gettrain_0309_doorLR) (Math|Vector|MakeVector (* _新規track_0 -1.0) 0.0 0.0) false false))))

(event Custom|Close_Door_Train_L
  ;[1 1 1] 電車左
  (bind _新規track_0 (Timeline|タイムライン_2 ReverseFromEnd)
    (:Update
      (Transformation|SetRelativeLocation (Variables|Default|Gettrain_0309_doorLL) (Math|Vector|MakeVector _新規track_0 0.0 0.0) false false)
      (Transformation|SetRelativeLocation (Variables|Default|Gettrain_0309_doorLR) (Math|Vector|MakeVector (* _新規track_0 -1.0) 0.0 0.0) false false))))

(fn ConstructionScript)