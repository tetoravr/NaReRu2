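; Plays in-train voice announcements for a Tokyo Metro ride bound for Ogikubo, covering stops from Shin-Otsuka to Tokyo.
; Each stop has a next-station event and an arrival event, each firing pre-placed sound components in sequence with fixed Delays.
; Arrivals add transfer notices where relevant and a Deguti (exit) call, except Tokyo.
; The Shin-Otsuka departure adds greeting, destination and sway-warning lines, and a separate event plays Omatase.
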(event Custom|Play_omatase
  (Class|AtomComponent|Play (Variables|Default|Getomatase) 0.0))

(event Custom|Play_announce_tokyo
  (Utilities|FlowControl|Delay 1e+01)
  (Class|AtomComponent|Play (Variables|Default|GetNext_tokyo) 0.0))

(event Custom|Play_announce_shinotsuka
  (Class|AtomComponent|Play (Variables|Default|Get東京メトロをご利用くださいましてありがとうございます。) 0.0)
  (Utilities|FlowControl|Delay 5.0)
  (Class|AtomComponent|Play (Variables|Default|Getこの電車は荻窪ゆきです) 0.0)
  (Utilities|FlowControl|Delay 5.0)
  (Class|AtomComponent|Play (Variables|Default|Getこの先揺れますのでご注意ください) 0.0)
  (Utilities|FlowControl|Delay 5.0)
  (Class|AtomComponent|Play (Variables|Default|GetNext_shinotsuka) 0.0)
  (Utilities|FlowControl|Delay 1e+01)
  (Class|AtomComponent|Play (Variables|Default|Getこの電車は荻窪ゆきです) 0.0))

(event Custom|到着_後楽園
  (Class|AtomComponent|Play (Variables|Default|GetSoon_korakuen) 0.0)
  (Utilities|FlowControl|Delay 3.0)
  (Class|AtomComponent|Play (Variables|Default|Get乗り換え_後楽園) 0.0)
  (Utilities|FlowControl|Delay 5.0)
  (Class|AtomComponent|Play (Variables|Default|Getdeguti) 0.0))

(event Custom|到着_東京
  (Class|AtomComponent|Play (Variables|Default|GetSoon_tokyo) 0.0))

(event Custom|到着_本郷三丁目
  (Class|AtomComponent|Play (Variables|Default|GetSoon_hongosanchome) 0.0)
  (Utilities|FlowControl|Delay 3.0)
  (Class|AtomComponent|Play (Variables|Default|Get乗り換え_本郷三丁目) 0.0)
  (Utilities|FlowControl|Delay 3.0)
  (Class|AtomComponent|Play (Variables|Default|Getdeguti) 0.0))

(event Custom|到着_御茶ノ水
  (Class|AtomComponent|Play (Variables|Default|GetSoon_ochanomizu) 0.0)
  (Utilities|FlowControl|Delay 3.0)
  (Class|AtomComponent|Play (Variables|Default|Getお茶ノ水乗り換え) 0.0)
  (Utilities|FlowControl|Delay 3.0)
  (Class|AtomComponent|Play (Variables|Default|Getdeguti) 0.0))

(event Custom|Play_announce_hongosanchome
  (Utilities|FlowControl|Delay 1e+01)
  (Class|AtomComponent|Play (Variables|Default|GetNext_hongosanchome) 0.0))

(event Custom|到着_淡路町
  (Class|AtomComponent|Play (Variables|Default|GetSoon_awajicho) 0.0)
  (Utilities|FlowControl|Delay 3.0)
  (Class|AtomComponent|Play (Variables|Default|Getdeguti) 0.0))

(event Custom|到着_大手町
  (Class|AtomComponent|Play (Variables|Default|GetSoon_otemachi) 0.0)
  (Utilities|FlowControl|Delay 3.0)
  (Class|AtomComponent|Play (Variables|Default|Get大手町乗り換え) 0.0)
  (Utilities|FlowControl|Delay 6.0)
  (Class|AtomComponent|Play (Variables|Default|Getdeguti) 0.0))

(event Custom|Play_announce_ochanomizu
  (Utilities|FlowControl|Delay 1e+01)
  (Class|AtomComponent|Play (Variables|Default|GetNext_ochanomizu) 0.0))

(event Custom|Play_announce_korakuen
  (Utilities|FlowControl|Delay 1e+01)
  (Class|AtomComponent|Play (Variables|Default|GetNext_korakuen) 0.0))

(event Custom|Play_announce_otemachi
  (Utilities|FlowControl|Delay 1e+01)
  (Class|AtomComponent|Play (Variables|Default|GetNext_otemachi) 0.0))

(event Custom|Play_announce_myogadani
  (Utilities|FlowControl|Delay 1e+01)
  (Class|AtomComponent|Play (Variables|Default|GetNext_myogadani) 0.0))

(event Custom|Play_announce_awajicho
  (Utilities|FlowControl|Delay 1e+01)
  (Class|AtomComponent|Play (Variables|Default|GetNext_awajicho) 0.0))

(event Custom|到着_新大塚
  (Class|AtomComponent|Play (Variables|Default|GetSoon_shinotsuka) 0.0)
  (Utilities|FlowControl|Delay 3.0)
  (Class|AtomComponent|Play (Variables|Default|Getdeguti) 0.0))

(event Custom|到着_茗荷谷
  (Class|AtomComponent|Play (Variables|Default|GetSoon_myogadani) 0.0)
  (Utilities|FlowControl|Delay 3.0)
  (Class|AtomComponent|Play (Variables|Default|Getdeguti) 0.0))

(fn ConstructionScript)