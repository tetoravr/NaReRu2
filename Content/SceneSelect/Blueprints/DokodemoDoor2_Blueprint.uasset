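; Anywhere-door actor for scene selection that changes its surface to represent a destination scene.
; Each scene has its own custom event, covering transport, speech, interview, elevator and thunder scenes.
; Every event swaps the first material slot of the static mesh to that scene's material.
; The Blueprint holds no travel or trigger logic, so the events rely on being called.
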(event Custom|Door_Airplane
  (Rendering|Material|SetMaterial (Variables|Debug|GetStaticMeshComponent) 0 "/Game/SceneSelect/Model/DokodemoDoor/Material/MI_Airplane.MI_Airplane"))

(event Custom|Door_Subway
  (Rendering|Material|SetMaterial (Variables|Debug|GetStaticMeshComponent) 0 "/Game/SceneSelect/Model/DokodemoDoor/Material/MI_Subway.MI_Subway"))

(event Custom|Door_Thunder
  (Rendering|Material|SetMaterial (Variables|Debug|GetStaticMeshComponent) 0 "/Game/SceneSelect/Model/DokodemoDoor/Material/MI_Thunder.MI_Thunder"))

(event Custom|Door_Interview
  (Rendering|Material|SetMaterial (Variables|Debug|GetStaticMeshComponent) 0 "/Game/SceneSelect/Model/DokodemoDoor/Material/MI_Interview.MI_Interview"))

(event Custom|Door_BulletTrain
  (Rendering|Material|SetMaterial (Variables|Debug|GetStaticMeshComponent) 0 "/Game/SceneSelect/Model/DokodemoDoor/Material/MI_BulletTrain.MI_BulletTrain"))

(event Custom|Door_SpeechRoom
  (Rendering|Material|SetMaterial (Variables|Debug|GetStaticMeshComponent) 0 "/Game/SceneSelect/Model/DokodemoDoor/Material/MI_SpeechRoom.MI_SpeechRoom"))

(event Custom|Door_Bus
  (Rendering|Material|SetMaterial (Variables|Debug|GetStaticMeshComponent) 0 "/Game/SceneSelect/Model/DokodemoDoor/Material/MI_Bus.MI_Bus"))

(event Custom|Door_Elevator
  (Rendering|Material|SetMaterial (Variables|Debug|GetStaticMeshComponent) 0 "/Game/SceneSelect/Model/DokodemoDoor/Material/MI_Elevator.MI_Elevator"))

(event Custom|Door_SpeechHall
  (Rendering|Material|SetMaterial (Variables|Debug|GetStaticMeshComponent) 0 "/Game/SceneSelect/Model/DokodemoDoor/Material/MI_ESpeechHall.MI_ESpeechHall"))

(event EventBeginPlay)

(event Collision|EventActorBeginOverlap
  (params (OtherActor :type Actor%20Object%20Reference)))

(event EventTick
  (params (DeltaSeconds :type Float%20%28single-precision%29)))

(fn ConstructionScript)