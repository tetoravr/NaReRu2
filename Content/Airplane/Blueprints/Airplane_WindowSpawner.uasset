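; Sequences the VR airplane scenario, from walking the patient aboard through takeoff and landing.
; A timeline moves the player and feeds progress to AirplaneWindow2 widgets, then fades and swaps the Plane streaming level for Plane_Flight.
; Delays time announcements, seatbelt lamp and beeps, with dispatcher calls signalling plane phases.
; Skip events jump into boarding completion or the DoOnce that enables takeoff.
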(event Custom|患者移動
  (bind _outactors (Actor|GetAllActorsOfClass "/Game/Airplane/Blueprints/Airplane_Sound_BP.Airplane_Sound_BP_C"))
  (for _array_element _outactors
    (bind _asairplane_sound_bp (Utilities|Casting|CastToAirplane_Sound_BP _array_element))
    (Default|PlaySoundAirplaneRecCrossfade _asairplane_sound_bp)
    ;[1 1 1] 患者移動
    (bind (_direction _プログレスバー _残り時間 _プレイヤー移動座標) (Timeline|タイムライン_0 Play)
      (:Update
        (bind _returnvalue (Actor|GetActorOfClass "/Game/NaReRu_Common/Blueprint/VR_Character/VRPlayer_Character.VRPlayer_Character_C"))
        (Transformation|SetActorLocationAndRotation _returnvalue (Math|Vector|MakeVector (.X (Math|Vector|BreakVector _プレイヤー移動座標)) (.Y (Math|Vector|BreakVector _プレイヤー移動座標)) (.Z (Math|Vector|BreakVector (Transformation|GetActorLocation (Game|GetPlayerCharacter 0))))) "0.0,-40.000000,0.0")
        ;[1 1 1] プログレスバー
        (bind _foundwidgets (Widget|GetAllWidgetsOfClass "/Game/Airplane/Blueprints/AirplaneWindow2.AirplaneWindow2_C" false))
        (for _array_element_2 _foundwidgets
          (Variables|/Game/Airplane/Blueprints/AirplaneWindow2.AirplaneWindow2_C|SetProgress _array_element_2 _プログレスバー)
          (Variables|/Game/Airplane/Blueprints/AirplaneWindow2.AirplaneWindow2_C|Set残り時間 _array_element_2 _残り時間)))
      (:Finished
        (Utilities|FlowControl|Sequence
          (:then_0
            (bind _foundwidgets_2 (Widget|GetAllWidgetsOfClass "/Game/Airplane/Blueprints/AirplaneWindow2.AirplaneWindow2_C" false))
            (for _array_element_3 _foundwidgets_2
              (Variables|/Game/Airplane/Blueprints/AirplaneWindow2.AirplaneWindow2_C|SetIsSit _array_element_3 true)
              ;[1 1 1] シーン切り替えとプレイヤー移動
              (CameraFades|StartCameraFade (Game|GetPlayerCameraManager 0) 0.0 1.0 5.0 "(R=1.000000,G=1.000000,B=1.000000,A=1.000000)" false false)
              (Utilities|FlowControl|Delay 5.1)
              (Game|LoadStreamLevel(byName) "Plane_Flight" true)
              (Transformation|SetActorLocationAndRotation (Game|GetPlayerCharacter 0) "-86220.000000,124450.000000,600.000000")
              (bind _outactors_2 (Actor|GetAllActorsOfClass "/Game/Airplane/Blueprints/PlaneGround.PlaneGround_C"))
              (Actor|DestroyActor _outactors_2)
              (Game|UnloadStreamLevel(byName) "Plane" false)
              (Default|Call飛行機ON)))
          (:then_1
            ;[1 1 1] 離陸前音声
            (bind _foundwidgets_3 (Widget|GetAllWidgetsOfClass "/Game/Airplane/Blueprints/AirplaneWindow2.AirplaneWindow2_C" false))
            (for _array_element_4 _foundwidgets_3
              (Variables|/Game/Airplane/Blueprints/AirplaneWindow2.AirplaneWindow2_C|SetAction _array_element_4 " アナウンス中")
              (Utilities|FlowControl|Delay 5.0)
              (if (not (Variables|Default|Get離陸))
                (Audio|Components|Audio|Play (Variables|Default|Get離陸前アナウンス) 0.0)
                (bind _残り時間_2 (Timeline|タイムライン_1 PlayFromStart)
                  (:Update
                    (|残り時間更新_2 _残り時間_2)
                    (Utilities|FlowControl|Delay 337.0)
                    (Utilities|FlowControl|DoOnce false
                      (:Completed
                        (bind _foundwidgets_4 (Widget|GetAllWidgetsOfClass "/Game/Airplane/Blueprints/AirplaneWindow2.AirplaneWindow2_C" false))
                        (Default|離陸有効化 _foundwidgets_4)))))))))))))

(event Custom|患者一時停止
  ;[1 1 1] 患者移動
  (bind (_direction _プログレスバー _残り時間 _プレイヤー移動座標) (Timeline|タイムライン_0 Stop)
    (:Update
      (bind _returnvalue (Actor|GetActorOfClass "/Game/NaReRu_Common/Blueprint/VR_Character/VRPlayer_Character.VRPlayer_Character_C"))
      (Transformation|SetActorLocationAndRotation _returnvalue (Math|Vector|MakeVector (.X (Math|Vector|BreakVector _プレイヤー移動座標)) (.Y (Math|Vector|BreakVector _プレイヤー移動座標)) (.Z (Math|Vector|BreakVector (Transformation|GetActorLocation (Game|GetPlayerCharacter 0))))) "0.0,-40.000000,0.0")
      ;[1 1 1] プログレスバー
      (bind _foundwidgets (Widget|GetAllWidgetsOfClass "/Game/Airplane/Blueprints/AirplaneWindow2.AirplaneWindow2_C" false))
      (for _array_element _foundwidgets
        (Variables|/Game/Airplane/Blueprints/AirplaneWindow2.AirplaneWindow2_C|SetProgress _array_element _プログレスバー)
        (Variables|/Game/Airplane/Blueprints/AirplaneWindow2.AirplaneWindow2_C|Set残り時間 _array_element _残り時間)))
    (:Finished
      (Utilities|FlowControl|Sequence
        (:then_0
          (bind _foundwidgets_2 (Widget|GetAllWidgetsOfClass "/Game/Airplane/Blueprints/AirplaneWindow2.AirplaneWindow2_C" false))
          (for _array_element_2 _foundwidgets_2
            (Variables|/Game/Airplane/Blueprints/AirplaneWindow2.AirplaneWindow2_C|SetIsSit _array_element_2 true)
            ;[1 1 1] シーン切り替えとプレイヤー移動
            (CameraFades|StartCameraFade (Game|GetPlayerCameraManager 0) 0.0 1.0 5.0 "(R=1.000000,G=1.000000,B=1.000000,A=1.000000)" false false)
            (Utilities|FlowControl|Delay 5.1)
            (Game|LoadStreamLevel(byName) "Plane_Flight" true)
            (Transformation|SetActorLocationAndRotation (Game|GetPlayerCharacter 0) "-86220.000000,124450.000000,600.000000")
            (bind _outactors (Actor|GetAllActorsOfClass "/Game/Airplane/Blueprints/PlaneGround.PlaneGround_C"))
            (Actor|DestroyActor _outactors)
            (Game|UnloadStreamLevel(byName) "Plane" false)
            (Default|Call飛行機ON)))
        (:then_1
          ;[1 1 1] 離陸前音声
          (bind _foundwidgets_3 (Widget|GetAllWidgetsOfClass "/Game/Airplane/Blueprints/AirplaneWindow2.AirplaneWindow2_C" false))
          (for _array_element_3 _foundwidgets_3
            (Variables|/Game/Airplane/Blueprints/AirplaneWindow2.AirplaneWindow2_C|SetAction _array_element_3 " アナウンス中")
            (Utilities|FlowControl|Delay 5.0)
            (if (not (Variables|Default|Get離陸))
              (Audio|Components|Audio|Play (Variables|Default|Get離陸前アナウンス) 0.0)
              (bind _残り時間_2 (Timeline|タイムライン_1 PlayFromStart)
                (:Update
                  (|残り時間更新_2 _残り時間_2)
                  (Utilities|FlowControl|Delay 337.0)
                  (Utilities|FlowControl|DoOnce false
                    (:Completed
                      (bind _foundwidgets_4 (Widget|GetAllWidgetsOfClass "/Game/Airplane/Blueprints/AirplaneWindow2.AirplaneWindow2_C" false))
                      (Default|離陸有効化 _foundwidgets_4))))))))))))

(event Custom|離陸ボタン
  ;[1 1 1] 離陸・着陸切り替え
  (Variables|Default|SetAnnounceVolume 0.0) ; アナウンスの音量を0にする
  (Development|SetHiddeninGame (Variables|Default|GetSkeletalMesh) true false)
  (Variables|Default|Set離陸 true)
  (Development|PrintString "離陸")
  (Default|Call飛行機離陸)
  (Utilities|FlowControl|Delay 9e+01)
  ;;[1 1 1] シートベルトのランプ
  (bind _returnvalue (Actor|GetActorOfClass "/Game/Airplane/Blueprints/SM_airbus_Lamp_2_Blueprint.SM_airbus_Lamp_2_Blueprint_C"))
  (Rendering|Material|SetMaterial (Variables|/Script/Engine.StaticMeshActor|GetStaticMeshComponent _returnvalue) 0 "/Game/Airplane/Object/Airbus/Material/LampOFF.LampOFF")
  (bind _returnvalue_2 (Actor|GetActorOfClass "/Game/Airplane/Blueprints/Airplane_Sound_BP.Airplane_Sound_BP_C"))
  (Default|PlaySoundAirplaneBeep _returnvalue_2)
  (Audio|Components|Audio|Play (Variables|Default|Get離陸後アナウンス) 0.0))

(event Custom|着陸ボタン
  ;[1 1 1] 離陸・着陸切り替え
  (Default|Call飛行機着陸) ; レベルブループリント
  (Utilities|FlowControl|Delay 1.0)
  (Audio|Components|Audio|Play (Variables|Default|Get着陸前アナウンス0) 0.0)
  (Utilities|FlowControl|Delay 3e+02)
  ;;[1 1 1] シートベルトランプ
  (bind _returnvalue (Actor|GetActorOfClass "/Game/Airplane/Blueprints/SM_airbus_Lamp_2_Blueprint.SM_airbus_Lamp_2_Blueprint_C"))
  (Rendering|Material|SetMaterial (Variables|/Script/Engine.StaticMeshActor|GetStaticMeshComponent _returnvalue) 0 "/Game/Airplane/Object/Airbus/Material/LampON.LampON")
  (bind _returnvalue_2 (Actor|GetActorOfClass "/Game/Airplane/Blueprints/Airplane_Sound_BP.Airplane_Sound_BP_C"))
  (Default|PlaySoundAirplaneBeep _returnvalue_2)
  (Utilities|FlowControl|Delay 1.0)
  (Audio|Components|Audio|Play (Variables|Default|Get着陸前アナウンス1) 0.0))

(event Custom|アナウンス_Skip
  ;[1 1 1] 離陸前音声
  (Audio|Components|Audio|SetVolumeMultiplier (Variables|Default|Get離陸前アナウンス) (Variables|Default|GetAnnounceVolume) :!class /Script/Engine.AudioComponent)
  (Utilities|FlowControl|DoOnce false
    (:Completed
      (bind _foundwidgets (Widget|GetAllWidgetsOfClass "/Game/Airplane/Blueprints/AirplaneWindow2.AirplaneWindow2_C" false))
      (Default|離陸有効化 _foundwidgets))))

(event Custom|搭乗スキップ
  (Utilities|FlowControl|Sequence
    (:then_0
      (bind _foundwidgets (Widget|GetAllWidgetsOfClass "/Game/Airplane/Blueprints/AirplaneWindow2.AirplaneWindow2_C" false))
      (for _array_element _foundwidgets
        (Variables|/Game/Airplane/Blueprints/AirplaneWindow2.AirplaneWindow2_C|SetIsSit _array_element true)
        ;[1 1 1] シーン切り替えとプレイヤー移動
        (CameraFades|StartCameraFade (Game|GetPlayerCameraManager 0) 0.0 1.0 5.0 "(R=1.000000,G=1.000000,B=1.000000,A=1.000000)" false false)
        (Utilities|FlowControl|Delay 5.1)
        (Game|LoadStreamLevel(byName) "Plane_Flight" true)
        (Transformation|SetActorLocationAndRotation (Game|GetPlayerCharacter 0) "-86220.000000,124450.000000,600.000000")
        (bind _outactors (Actor|GetAllActorsOfClass "/Game/Airplane/Blueprints/PlaneGround.PlaneGround_C"))
        (Actor|DestroyActor _outactors)
        (Game|UnloadStreamLevel(byName) "Plane" false)
        (Default|Call飛行機ON)))
    (:then_1
      ;[1 1 1] 離陸前音声
      (bind _foundwidgets_2 (Widget|GetAllWidgetsOfClass "/Game/Airplane/Blueprints/AirplaneWindow2.AirplaneWindow2_C" false))
      (for _array_element_2 _foundwidgets_2
        (Variables|/Game/Airplane/Blueprints/AirplaneWindow2.AirplaneWindow2_C|SetAction _array_element_2 " アナウンス中")
        (Utilities|FlowControl|Delay 5.0)
        (if (not (Variables|Default|Get離陸))
          (Audio|Components|Audio|Play (Variables|Default|Get離陸前アナウンス) 0.0)
          (bind _残り時間 (Timeline|タイムライン_1 PlayFromStart)
            (:Update
              (|残り時間更新_2 _残り時間)
              (Utilities|FlowControl|Delay 337.0)
              (Utilities|FlowControl|DoOnce false
                (:Completed
                  (bind _foundwidgets_3 (Widget|GetAllWidgetsOfClass "/Game/Airplane/Blueprints/AirplaneWindow2.AirplaneWindow2_C" false))
                  (Default|離陸有効化 _foundwidgets_3))))))))))

(event EventBeginPlay)

(fn ConstructionScript)