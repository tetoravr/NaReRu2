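; ChangeLevel_BP controls audience reactions in a speech scene, setting animation level and reaction flags.
; Attitude events set one of four AnimationLevel steps, while agree and anger events raise flags, each holding Input true for a timed delay.
; Applause plays hall or room clap audio by current level name, with timelines driving volume.
; When applause ends or the listen event fires, flags clear and SpeechWindow widgets get their attitude reset.
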(event Custom|拍手
  (bind _clap_hall (Variables|Default|GetClap_Hall))
  (bind _clap_room (Variables|Default|GetClap_Room))
  (Variables|Default|SetClap true) ; 拍手
  (Variables|Default|SetInput true)
  (bind _returnvalue (Game|GetCurrentLevelName true))
  (switch string _returnvalue
    (:ConferenceHall
      (Audio|Components|Audio|Play (Variables|Default|GetClap_Hall) 0.0)
      (bind _音量 (Timeline|タイムライン_0 PlayFromStart)
        (:Update
          (Audio|Components|Audio|SetVolumeMultiplier _clap_hall _音量 :!class /Script/Engine.AudioComponent))
        (:Finished
          (Variables|Default|SetInput false)
          (Variables|Default|SetClap false) ; 拍手
          (bind _foundwidgets (Widget|GetAllWidgetsOfClass "/Game/Speech/Blueprint/SpeechWindow.SpeechWindow_C" false))
          (Default|態度初期 _foundwidgets)
          (Audio|Components|Audio|Stop _clap_hall))))
    (:ConferenceRoom_Master
      (Audio|Components|Audio|Play _clap_room 0.0)
      (bind _音量_2 (Timeline|タイムライン_1 PlayFromStart)
        (:Update
          (Audio|Components|Audio|SetVolumeMultiplier _clap_room _音量_2 :!class /Script/Engine.AudioComponent))
        (:Finished
          (Audio|Components|Audio|Stop _clap_room))
        (:新規Track_0
          (Variables|Default|SetInput false)
          (Variables|Default|SetClap false) ; 拍手
          (bind _foundwidgets_2 (Widget|GetAllWidgetsOfClass "/Game/Speech/Blueprint/SpeechWindow.SpeechWindow_C" false))
          (Default|態度初期 _foundwidgets_2))))))

(event Custom|態度0
  (Variables|Default|SetAnimationLevel 100)
  (Variables|Default|SetInput true)
  (Development|PrintString "100%")
  (Utilities|FlowControl|Delay 5.0)
  (Variables|Default|SetInput false))

(event Custom|態度1
  (Variables|Default|SetAnimationLevel 50)
  (Variables|Default|SetInput true)
  (Development|PrintString "50%")
  (Utilities|FlowControl|Delay 5.0)
  (Variables|Default|SetInput false))

(event Custom|態度2
  (Variables|Default|SetAnimationLevel 20)
  (Variables|Default|SetInput true)
  (Development|PrintString "20%")
  (Utilities|FlowControl|Delay 5.0)
  (Variables|Default|SetInput false))

(event Custom|態度3
  (Variables|Default|SetAnimationLevel 0)
  (Variables|Default|SetInput true)
  (Development|PrintString "0%")
  (Utilities|FlowControl|Delay 5.0)
  (Variables|Default|SetInput false))

(event Custom|清聴
  (Variables|Default|SetInput false)
  (Variables|Default|SetClap false) ; 拍手
  (bind _foundwidgets (Widget|GetAllWidgetsOfClass "/Game/Speech/Blueprint/SpeechWindow.SpeechWindow_C" false))
  (Default|態度初期 _foundwidgets))

(event Custom|同意
  (Variables|Default|Setagree true)
  (Variables|Default|SetInput true)
  (Utilities|FlowControl|Delay 2.0)
  (Variables|Default|SetInput false)
  (Variables|Default|Setagree false)
  (Variables|Default|Setanger false))

(event Custom|怒る
  (Variables|Default|Setanger true)
  (Variables|Default|SetInput true)
  (Utilities|FlowControl|Delay 2.0)
  (Variables|Default|SetInput false)
  (Variables|Default|Setagree false)
  (Variables|Default|Setanger false))

(event EventBeginPlay
  (Variables|Default|SetAnimationLevel 100)
  (Variables|Default|SetInput true)
  (Development|PrintString "100%")
  (Utilities|FlowControl|Delay 5.0)
  (Variables|Default|SetInput false))

(fn ConstructionScript)