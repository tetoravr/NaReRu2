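; Bullet train Blueprint that sets up a 960x1000 window and provides events for seating and moving the VR player.
; BeginPlay applies the resolution by console command, and the sit event changes the VRPlayer_Character camera height from SitHight before calling its height update.
; The move event drives the player's location with a timeline, then fades the camera to white and opens the shinkansenrun level.
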(event Custom|プレイヤー移動
  (bind _returnvalue (Game|GetPlayerCharacter 0))
  (bind _新規track_0 (Timeline|タイムライン_0 Play)
    (:Update
      (Transformation|SetActorLocationAndRotation _returnvalue (+ _新規track_0 (Math|Conversions|ToVector(Float) (.Z (Math|Vector|BreakVector (Transformation|GetActorLocation _returnvalue)))))))
    (:Finished
      (CameraFades|StartCameraFade (Game|GetPlayerCameraManager 0) 0.0 1.0 5.0 "(R=1.000000,G=1.000000,B=1.000000,A=1.000000)" false false)
      (Utilities|FlowControl|Delay 5.0)
      (Game|OpenLevel(byName) "shinkansenrun"))))

(event Custom|座る
  ;[1 1 1] 座ったときの視点変更
  (bind _returnvalue (Actor|GetActorOfClass "/Game/NaReRu_Common/Blueprint/VR_Character/VRPlayer_Character.VRPlayer_Character_C"))
  (Variables|/Game/NaReRu_Common/Blueprint/VR_Character/VRPlayer_Character.VRPlayer_Character_C|SetVRCameraHight _returnvalue (+ (Variables|Default|GetSitHight) 5e+01))
  (Default|身長変更 _returnvalue))

(event EventBeginPlay
  (Development|ExecuteConsoleCommand (Utilities|String|MakeLiteralString "r.SetRes 960x1000w") 0))

(fn ConstructionScript)