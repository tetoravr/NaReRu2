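; Spawner actor that keeps producing right-side cars (RightSideCar_Blueprint) for the duration of play.
; On BeginPlay it picks one of four scene components at random and spawns a car at that component's world transform.
; It then waits a random 3 to 10 seconds and loops back through the Delay to spawn again indefinitely.
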(event EventBeginPlay
  (switch int (Math|Random|RandomIntegerinRange 0 3) :!label _label
    (:0
      (Game|SpawnActorfromClass "/Game/Elevator/Blueprint/RightSideCar_Blueprint.RightSideCar_Blueprint_C" (Transformation|GetWorldTransform (Variables|Default|GetScene1)) "Undefined" 0 0))
    (:1
      (Game|SpawnActorfromClass "/Game/Elevator/Blueprint/RightSideCar_Blueprint.RightSideCar_Blueprint_C" (Transformation|GetWorldTransform (Variables|Default|GetScene2)) "Undefined" 0 0))
    (:2
      (Game|SpawnActorfromClass "/Game/Elevator/Blueprint/RightSideCar_Blueprint.RightSideCar_Blueprint_C" (Transformation|GetWorldTransform (Variables|Default|GetScene3)) "Undefined" 0 0))
    (:3
      (Game|SpawnActorfromClass "/Game/Elevator/Blueprint/RightSideCar_Blueprint.RightSideCar_Blueprint_C" (Transformation|GetWorldTransform (Variables|Default|GetScene)) "Undefined" 0 0)))
  (Utilities|FlowControl|Delay (Math|Random|RandomFloatinRange 3.0 1e+01))
  (goto _label))

(event Collision|EventActorBeginOverlap
  (params (OtherActor :type Actor%20Object%20Reference)))

(event EventTick
  (params (DeltaSeconds :type Float%20%28single-precision%29)))

(fn ConstructionScript)