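; Spectator-window actor for the elevator content that sets the display resolution and relays the start of patient movement (患者移動).
; BeginPlay runs an r.SetRes console command to set a fixed windowed resolution.
; The 患者移動 event calls 患者移動開始, noted as bound for the Level Blueprint.
; Unconnected leftover nodes cover widget lookup, actor visibility, timeline-driven player movement and delayed door opening, none of which run.
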(event Custom|患者移動
  (Default|Call患者移動開始) ; レベルブループリント
)

(event EventBeginPlay
  (Development|ExecuteConsoleCommand (Utilities|String|MakeLiteralString "r.SetRes 960x1000w") 0))

(fn ConstructionScript)