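; Elevator button Blueprint, placed as a child actor of BP_Elevator_Box, that queues a floor and lights up.
; The 上昇開始 (start ascent) event passes NextFloor from every ElevatorWindow2 widget to the parent's AddToFloorQueue, calling TurnOn for each.
; TurnOn and TurnOff swap the lit and unlit materials on slot 1 of the button mesh, which the construction script assigns.
; BeginPlay and PressButton are empty.
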(event Custom|上昇開始
  ;[1 1 1] ボタンを押す --> フロア番号をキューに追加する
  (bind _foundwidgets (Widget|GetAllWidgetsOfClass "/Game/Elevator/Blueprint/ElevatorWindow2.ElevatorWindow2_C" false))
  (bind _asbp_elevator_box (Utilities|Casting|CastToBP_Elevator_Box (Actor|GetParentActor)))
  (for _array_element _foundwidgets
    (Default|AddtoFloorQueue _asbp_elevator_box (Variables|/Game/Elevator/Blueprint/ElevatorWindow2.ElevatorWindow2_C|GetNextFloor _array_element))
    (CallFunction|Turnon)))

(event Custom|PressButton)

(event Custom|TurnOff
  ;[1 1 1] Turn Off --> Change Material to UNLIT
  (Rendering|Material|SetMaterial (Variables|Default|Getsm_buttons_floor_button-1) 1 (Variables|Default|GetmaterialOff)))

(event Custom|TurnOn
  ;[1 1 1] Turn On --> Change Material to LIT version
  (Rendering|Material|SetMaterial (Variables|Default|Getsm_buttons_floor_button-1) 1 (Variables|Default|GetmaterialOn)))

(event EventBeginPlay)

(fn ConstructionScript
  (Components|StaticMesh|SetStaticMesh (Variables|Default|Getsm_buttons_floor_button-1) (Variables|Default|GetstaticMeshButton)))