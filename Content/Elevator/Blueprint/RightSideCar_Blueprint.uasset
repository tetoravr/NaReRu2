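; Right-side car actor that appears as one of five random mesh variants and drives continuously along world +X.
; BeginPlay hides all five static meshes, then unhides one chosen at random.
; Tick moves the actor by a fixed, unswept step each frame, independent of frame rate.
; Its destroy check compares single-frame DeltaSeconds to a large threshold rather than accumulated lifetime, so it effectively never fires.
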(event EventBeginPlay
  (Development|SetHiddeninGame (Variables|Default|GetStaticMesh1) true false)
  (switch int (Math|Random|RandomIntegerinRange 0 4)
    (:0
      (Development|SetHiddeninGame (Variables|Default|GetStaticMesh1) false false))
    (:1
      (Development|SetHiddeninGame (Variables|Default|GetStaticMesh2) false false))
    (:2
      (Development|SetHiddeninGame (Variables|Default|GetStaticMesh3) false false))
    (:3
      (Development|SetHiddeninGame (Variables|Default|GetStaticMesh4) false false))
    (:4
      (Development|SetHiddeninGame (Variables|Default|GetStaticMesh) false false))))

(event Collision|EventActorBeginOverlap
  (params (OtherActor :type Actor%20Object%20Reference)))

(event EventTick
  (params (DeltaSeconds :type Float%20%28single-precision%29))
  (Transformation|SetActorLocation (+ (Transformation|GetActorLocation) "25.000000, 0,0.000000") false false)
  (if (>= DeltaSeconds 5e+01)
    (Actor|DestroyActor)))

(fn ConstructionScript)