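; BP_TopFrame is the top frame of an elevator system, animating the cables and counterweight as the elevator box moves.
; On BeginPlay it caches the box from the system's child actor and the cable mesh's anim Blueprint, then records the initial cable-to-box height.
; Each Tick it feeds the anim Blueprint the offset to the box's attachment point and a counterweight value derived from the change in that height.
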(event EventBeginPlay
  (bind _elevatorsystem (Variables|Default|GetelevatorSystem))
  (bind _elevator_box (Variables|/Game/Elevator/Blueprint/BP_Elevator_System.BP_Elevator_System_C|GetElevator_Box _elevatorsystem))
  (bind _childactor (Variables|/Script/Engine.ChildActorComponent|GetChildActor _elevator_box))
  ;[1 1 1] Initialize variables
  (Utilities|IsValid _childactor
    (:Is%20Valid
      (bind _asbp_elevator_box (Utilities|Casting|CastToBP_Elevator_Box _childactor))
      (Variables|Default|SetelevatorBox _asbp_elevator_box)
      (bind _asbp_animation_cable_system (Utilities|Casting|CastToBP_AnimationCableSystem (Components|SkeletalMesh|GetAnimInstance (Variables|Default|Getsk_cableSystem))))
      (Variables|Default|SetcableSystemAnimBP _asbp_animation_cable_system)
      (Variables|Default|SetelevatorTotalHeight (.Z (Math|Vector|BreakVector (- (Transformation|GetWorldLocation (Variables|Default|Getsk_cableSystem)) (Transformation|GetWorldLocation (Variables|/Game/Elevator/Blueprint/BP_Elevator_Box.BP_Elevator_Box_C|GetcableAttachmentPoint (Variables|Default|GetelevatorBox))))))))))

(event EventTick
  (params (DeltaSeconds :type Float%20%28single-precision%29))
  (bind _cablesystemanimbp (Variables|Default|GetcableSystemAnimBP))
  ;[1 1 1] Move the cable wires so they follow the elevator box;
  ; Move the counter weight in accordance to the elevator box's position
  (Variables|/Game/Elevator/Blueprint/BP_AnimationCableSystem.BP_AnimationCableSystem_C|SetcableAttachmentPoint _cablesystemanimbp (* (- (Transformation|GetWorldLocation (Variables|Default|Getsk_cableSystem)) (Transformation|GetWorldLocation (Variables|/Game/Elevator/Blueprint/BP_Elevator_Box.BP_Elevator_Box_C|GetcableAttachmentPoint (Variables|Default|GetelevatorBox)))) -1.0))
  (Variables|/Game/Elevator/Blueprint/BP_AnimationCableSystem.BP_AnimationCableSystem_C|SetcounterWeight _cablesystemanimbp (* (- (Variables|Default|GetelevatorTotalHeight) (.Z (Math|Vector|BreakVector (- (Transformation|GetWorldLocation (Variables|Default|Getsk_cableSystem)) (Transformation|GetWorldLocation (Variables|/Game/Elevator/Blueprint/BP_Elevator_Box.BP_Elevator_Box_C|GetcableAttachmentPoint (Variables|Default|GetelevatorBox))))))) -1.0)))

(fn ConstructionScript)