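; Interview character Blueprint that animates a seated skeletal mesh during a job-interview simulation.
; The interview-start event steps the AnimBP's SitAnimValue through timed sit stages, and the questioning event switches it after a short delay; the end event is empty.
; Graphs gather question voice clips and sequences in four tones (normal, gentle, harsh, pressure), but none are used.
; Lip-sync and blink morph-target logic exists but never runs.
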(event Custom|面接開始
  (bind _asinterview_animation_bp (Utilities|Casting|CastToInterview_AnimationBP (Components|SkeletalMesh|GetAnimInstance (Variables|SkeletalMeshActor|GetSkeletalMeshComponent))))
  (Variables|/Game/Interview/Animaiton/Interview_AnimationBP.Interview_AnimationBP_C|SetSitAnimValue _asinterview_animation_bp 1)
  (Utilities|FlowControl|Delay 1.5)
  (Variables|/Game/Interview/Animaiton/Interview_AnimationBP.Interview_AnimationBP_C|SetSitAnimValue _asinterview_animation_bp 2)
  (Utilities|FlowControl|Delay 0.7)
  (Variables|/Game/Interview/Animaiton/Interview_AnimationBP.Interview_AnimationBP_C|SetSitAnimValue _asinterview_animation_bp 3))

(event Custom|面接終了)

(event Custom|質問中
  (Utilities|FlowControl|Delay 1.0)
  (bind _asinterview_animation_bp (Utilities|Casting|CastToInterview_AnimationBP (Components|SkeletalMesh|GetAnimInstance (Variables|SkeletalMeshActor|GetSkeletalMeshComponent))))
  (Variables|/Game/Interview/Animaiton/Interview_AnimationBP.Interview_AnimationBP_C|SetSitAnimValue _asinterview_animation_bp 5))

(fn ConstructionScript)