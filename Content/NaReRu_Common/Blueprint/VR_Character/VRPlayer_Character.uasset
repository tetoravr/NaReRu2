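; VR player character that handles camera height, headset setup and performance settings at startup.
; BeginPlay hides the body mesh and resets eye-level tracking, then joins the height-change (身長変更) path to offset VRCameraRoot.
; That path triggers VR初期化, which applies delayed console commands for resolution scale and frame cap, and sets windowed 1080p, identically for Login and other levels.
; A 体表示 event toggles body visibility.
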(event Custom|体表示
  (Utilities|FlowControl|FlipFlop
    (:A
      (Development|SetHiddeninGame (Variables|Default|GetSkeletalMesh) false false))
    (:B
      (Development|SetHiddeninGame (Variables|Default|GetSkeletalMesh) true false))))

(event Custom|身長変更
  ;[1 1 1] Offset the VRCameraRoot to move the Vive Camera
  (Transformation|SetRelativeLocation (Variables|Default|GetVRCameraRoot) (Math|Vector|MakeVector 0.0 0.0 (Variables|Default|GetVRCameraHight)) false false)
  (CallFunction|VR初期化)
  (bind _returnvalue (Game|GetCurrentLevelName true))
  (switch string _returnvalue
    (:Default
      (bind _returnvalue_2 (Settings|GetGameUserSettings))
      (Class|GameUserSettings|SetDynamicResolutionEnabled _returnvalue_2 true)
      (Class|GameUserSettings|ApplyNonResolutionSettings _returnvalue_2)
      (Class|GameUserSettings|SetFullscreenMode _returnvalue_2 "Windowed")
      (Class|GameUserSettings|SetScreenResolution _returnvalue_2 (Utilities|Struct|MakeIntPoint 1920 1080))
      (Class|GameUserSettings|ApplySettings _returnvalue_2 true))
    (:Login
      (bind _returnvalue_3 (Settings|GetGameUserSettings))
      (Class|GameUserSettings|SetDynamicResolutionEnabled _returnvalue_3 true)
      (Class|GameUserSettings|ApplyNonResolutionSettings _returnvalue_3)
      (Class|GameUserSettings|SetFullscreenMode _returnvalue_3 "Windowed")
      (Class|GameUserSettings|SetScreenResolution _returnvalue_3 (Utilities|Struct|MakeIntPoint 1920 1080))
      (Class|GameUserSettings|ApplySettings _returnvalue_3 true))))

(event Custom|VR初期化
  (Utilities|FlowControl|Delay 0.5)
  (Development|ExecuteConsoleCommand "hmd pd 0.6" 0)
  (Development|ExecuteConsoleCommand "r.ScreenPercentage 70" 0)
  (Development|ExecuteConsoleCommand "t.maxFPS 120" 0)
  (Development|ExecuteConsoleCommand "r.SceneRenderTargetResizeMethod 2" 0))

(event EventTick
  (params (DeltaSeconds :type Float%20%28single-precision%29)))

(event EventBeginPlay
  (Development|SetHiddeninGame (Variables|Default|GetSkeletalMesh) true false)
  (Class|HeadMountedDisplayFunctionLibrary|SetTrackingOrigin "Eye")
  (Class|HeadMountedDisplayFunctionLibrary|ResetOrientationandPosition 0.0 "OrientationAndPosition")
  ;[1 1 1] Offset the VRCameraRoot to move the Vive Camera
  (Transformation|SetRelativeLocation (Variables|Default|GetVRCameraRoot) (Math|Vector|MakeVector 0.0 0.0 (Variables|Default|GetVRCameraHight)) false false)
  (CallFunction|VR初期化)
  (bind _returnvalue (Game|GetCurrentLevelName true))
  (switch string _returnvalue
    (:Default
      (bind _returnvalue_2 (Settings|GetGameUserSettings))
      (Class|GameUserSettings|SetDynamicResolutionEnabled _returnvalue_2 true)
      (Class|GameUserSettings|ApplyNonResolutionSettings _returnvalue_2)
      (Class|GameUserSettings|SetFullscreenMode _returnvalue_2 "Windowed")
      (Class|GameUserSettings|SetScreenResolution _returnvalue_2 (Utilities|Struct|MakeIntPoint 1920 1080))
      (Class|GameUserSettings|ApplySettings _returnvalue_2 true))
    (:Login
      (bind _returnvalue_3 (Settings|GetGameUserSettings))
      (Class|GameUserSettings|SetDynamicResolutionEnabled _returnvalue_3 true)
      (Class|GameUserSettings|ApplyNonResolutionSettings _returnvalue_3)
      (Class|GameUserSettings|SetFullscreenMode _returnvalue_3 "Windowed")
      (Class|GameUserSettings|SetScreenResolution _returnvalue_3 (Utilities|Struct|MakeIntPoint 1920 1080))
      (Class|GameUserSettings|ApplySettings _returnvalue_3 true))))

(fn ConstructionScript)